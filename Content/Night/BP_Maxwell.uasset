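; BP_Maxwell is an actor that plays the Maxwell sound on begin play and wobbles from side to side.
; Each tick it rolls at a constant rate in the direction held by RollDir, keeping pitch and yaw unchanged.
; When roll passes a fixed limit either way, it updates RollDir and snaps the roll to that limit, signed by the direction, to produce the back-and-forth rocking.
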(event EventBeginPlay
  (Audio|PlaySound2D "/Game/Night/S_Maxwell.S_Maxwell" 1.0 1.0 0.0 0 0))

(event EventTick
  (params (DeltaSeconds :type Float%20%28single-precision%29))
  (bind _returnvalue (Transformation|GetActorRotation))
  (bind _returnvalue_2 (Transformation|GetActorRotation))
  (Transformation|SetActorRotation (Math|Rotator|MakeRotator (+ (* DeltaSeconds 135.0 (Variables|Default|GetRoll%20Dir)) (.roll _returnvalue)) (.pitch _returnvalue) (.yaw _returnvalue)))
  (if (> (Math|Float|Absolute(Float) (.roll _returnvalue_2)) 3e+01)
    (Math|Float|NegateFloat (Variables|Default|GetRoll%20Dir)
      (:%20%20
        (Transformation|SetActorRotation (Math|Rotator|MakeRotator (* -3e+01 (Variables|Default|GetRoll%20Dir)) (.pitch _returnvalue_2) (.yaw _returnvalue_2)))))))

(fn ConstructionScript)