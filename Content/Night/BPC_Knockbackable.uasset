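; Actor component that lets its owning Character be knocked back, scaled by a knockback resistance percentage.
; On BeginPlay it turns the resistance into a power multiplier, caches the owner as a Character and binds to its landed event.
; KnockBack launches the character with the scaled vector and sets its capsule to ignore the Pawn channel, which is restored to Block on landing.
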(event Custom|On%20Landed
  (params (Hit :type Hit%20Result%20Structure%20%28by%20ref%29))
  (Collision|SetCollisionResponsetoChannel (Variables|/Script/Engine.Character|GetCapsuleComponent (Variables|Default|GetOwner%20Char)) "ECC_Pawn" "ECR_Block"))

(event EventBeginPlay
  (Utilities|FlowControl|Sequence
    (:then_0
      (Variables|Default|SetKB%20Power%20Mult (- 1.0 (/ (Variables|Knockbackable|GetKnockback%20Resistence%20%25) 1e+02))))
    (:then_1
      (bind _ascharacter (Utilities|Casting|CastToCharacter (Components|GetOwner)))
      (Variables|Default|SetOwner%20Char _ascharacter))
    (:then_2
      (EventDispatchers|BindEventtoLandedDelegate (Variables|Default|GetOwner%20Char) (delegate Custom|On%20Landed)))))

(fn KnockBack
  (params (Knockback%20Vec :type Vector))
  (bind _owner_char (Variables|Default|GetOwner%20Char))
  (Collision|SetCollisionResponsetoChannel (Variables|/Script/Engine.Character|GetCapsuleComponent _owner_char) "ECC_Pawn" "ECR_Ignore")
  (Character|LaunchCharacter _owner_char (* Knockback%20Vec (Variables|Default|GetKB%20Power%20Mult)) false false))