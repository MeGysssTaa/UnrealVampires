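; GM_Night is the night game mode that spawns the player as the hero class stored on the game instance.
; Its construction script casts the game instance to GI_Undeads and caches it.
; Both default pawn spawn overrides, by start spot and by transform, spawn that SelectedHeroClass actor instead of a fixed default pawn.
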(fn ConstructionScript
  (bind _asgi_undeads (Utilities|Casting|CastToGI_Undeads (Game|GetGameInstance)))
  (Variables|Default|SetMy%20Game%20Instance _asgi_undeads))

(fn SpawnDefaultPawnatTransform
  (params (NewPlayer :type Controller%20Object%20Reference) (SpawnTransform :type Transform%20%28by%20ref%29))
  (bind _returnvalue (Game|SpawnActorfromClass (Variables|/Game/City/GI_Undeads.GI_Undeads_C|GetSelected%20Hero%20Class (Variables|Default|GetMy%20Game%20Instance)) SpawnTransform "Undefined" 0 0))
  (return _returnvalue))

(fn SpawnDefaultPawnfor
  (params (NewPlayer :type Controller%20Object%20Reference) (StartSpot :type Actor%20Object%20Reference))
  (bind _returnvalue (Game|SpawnActorfromClass (Variables|/Game/City/GI_Undeads.GI_Undeads_C|GetSelected%20Hero%20Class (Variables|Default|GetMy%20Game%20Instance)) (Transformation|GetActorTransform StartSpot) "Undefined" 0 0))
  (return _returnvalue))