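; BPC_Living is an actor component that gives its owner health, damage handling and a floating health bar.
; On BeginPlay it spawns and attaches a BP_Living_Actor, caches that actor's UI_HealthBar widget, fills health and binds the owner's OnTakeAnyDamage.
; Damage routes into Hurt, which clamps health at zero and sends KillLivingMessage with an impulse to the owner on death.
; Hurt, Heal and SetMaxHealth each refresh the bar.
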(event Custom|On%20Any%20Damage
  (params (DamagedActor :type Actor%20Object%20Reference) (Damage :type Float%20%28single-precision%29) (DamageType :type Damage%20Type%20Object%20Reference) (InstigatedBy :type Controller%20Object%20Reference) (DamageCauser :type Actor%20Object%20Reference))
  (CallFunction|Hurt Damage "0, 0, 0"))

(event EventBeginPlay
  (Utilities|FlowControl|Sequence
    (:then_0
      (bind _returnvalue (Game|SpawnActorfromClass "/Game/Night/BP_Living_Actor.BP_Living_Actor_C" (Math|Transform|MakeTransform "0, 0, 0" "0, 0, 0" "1.000000,1.000000,1.000000") "Undefined" 0 0))
      (Transformation|AttachActorToActor _returnvalue (Components|GetOwner) "None" "KeepRelative" "KeepRelative" "KeepRelative" true)
      (bind _output_get (Variables|Default|SetLiving%20Actor _returnvalue))
      (bind _asui_health_bar (Utilities|Casting|CastToUI_HealthBar (UserInterface|GetWidget (Variables|/Game/Night/BP_Living_Actor.BP_Living_Actor_C|GetWidget _output_get))))
      (Variables|Default|SetHealth%20Bar _asui_health_bar))
    (:then_1
      (Variables|Default|SetHealth (Variables|Default|GetMax%20Health))
      (CallFunction|UpdateUI))
    (:then_2
      (EventDispatchers|BindEventtoOnTakeAnyDamage (Components|GetOwner) (delegate Custom|On%20Any%20Damage)))))

(event EventTick
  (params (DeltaSeconds :type Float%20%28single-precision%29)))

(event EventEndPlay
  (params (EndPlayReason :type EEndPlayReason%20Enum :default "Destroyed")))

(fn Hurt
  (params (Damage%20Amount :type Float%20%28double-precision%29) (Kill%20Impulse :type Vector))
  (Variables|Default|SetHealth (Math|Float|Max(Float) (- (Variables|Default|GetHealth) Damage%20Amount) 0.0))
  (CallFunction|UpdateUI)
  (if (<= (Variables|Default|GetHealth) 0.0)
    (Class|BPILiving|KillLiving(Message) (Components|GetOwner) Kill%20Impulse)))

(fn UpdateUI
  (Progress|SetPercent (Variables|/Game/Night/UI_HealthBar.UI_HealthBar_C|GetHealthBar (Variables|Default|GetHealth%20Bar)) (/ (Variables|Default|GetHealth) (Variables|Default|GetMax%20Health))))

(fn GetHealth
  (return (Variables|Default|GetHealth)))

(fn SetMaxHealth
  (params (New%20Max%20Health :type Float%20%28double-precision%29) (Reset%20Current%20Health :type Boolean))
  (Variables|Default|SetMax%20Health New%20Max%20Health)
  (if Reset%20Current%20Health
    (Variables|Default|SetHealth (Variables|Default|GetMax%20Health)))
  (CallFunction|UpdateUI))

(fn Heal
  (params (Heal%20Amount :type Float%20%28double-precision%29))
  (Variables|Default|SetHealth (Math|Float|Min(Float) (+ (Variables|Default|GetHealth) Heal%20Amount) (Variables|Default|GetMax%20Health)))
  (CallFunction|UpdateUI))