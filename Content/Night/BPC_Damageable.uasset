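; Actor component that gives its owner health, with hurt and heal functions, and displays it on a floating health bar.
; On BeginPlay it spawns a helper actor attached to the owner and takes the health bar widget from it.
; Hurt sends KillItMessage with an impulse to the owner at zero health.
; Tick shrinks a recent-damage bar toward current health, colored by damage size, and fades the bar out once removal starts.
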(event EventBeginPlay
  (Utilities|FlowControl|Sequence
    (:then_0
      (bind _returnvalue (Game|SpawnActorfromClass "/Game/Night/BP_Damageable_Actor.BP_Damageable_Actor_C" (Math|Transform|MakeTransform "0, 0, 0" "0, 0, 0" "1.000000,1.000000,1.000000") "Undefined" 0 0))
      (Transformation|AttachActorToActor _returnvalue (Components|GetOwner) "None" "KeepRelative" "KeepRelative" "KeepRelative" true)
      (bind _output_get (Variables|Default|SetHealth%20Bar%20Holder%20Actor _returnvalue))
      (bind _asui_health_bar (Utilities|Casting|CastToUI_HealthBar (UserInterface|GetWidget (Variables|/Game/Night/BP_Damageable_Actor.BP_Damageable_Actor_C|GetWidget _output_get))))
      (Variables|Default|SetHealth%20Bar _asui_health_bar))
    (:then_1
      (Variables|Default|SetHealth (Variables|Default|GetMax%20Health))
      (CallFunction|UpdateDisplayedHealth))))

(event EventTick
  (params (DeltaSeconds :type Float%20%28single-precision%29))
  (CallFunction|TickRecentDamageAnimation)
  (if (Variables|Default|GetIs%20Being%20Removed)
    (CallFunction|TickRemovalAnimation)))

(fn Hurt
  (params (Damage%20Amount :type Float%20%28double-precision%29) (Kill%20Impulse :type Vector))
  (Variables|Default|SetHealth (Math|Float|Max(Float) (- (Variables|Default|GetHealth) Damage%20Amount) 0.0))
  (CallFunction|UpdateDisplayedHealth)
  (if (<= (Variables|Default|GetHealth) 0.0)
    (Class|BPIKillable|KillIt(Message) (Components|GetOwner) Kill%20Impulse)))

(fn UpdateDisplayedHealth
  (Progress|SetPercent (Variables|/Game/Night/UI_HealthBar.UI_HealthBar_C|GetHealthBar (Variables|Default|GetHealth%20Bar)) (/ (Variables|Default|GetHealth) (Variables|Default|GetMax%20Health))))

(fn GetHealth
  (return (Variables|Default|GetHealth)))

(fn SetMaxHealth
  (params (New%20Max%20Health :type Float%20%28double-precision%29) (Reset%20Current%20Health :type Boolean))
  (Variables|Default|SetMax%20Health New%20Max%20Health)
  (if Reset%20Current%20Health
    (Variables|Default|SetHealth (Variables|Default|GetMax%20Health)))
  (CallFunction|UpdateDisplayedHealth))

(fn Heal
  (params (Heal%20Amount :type Float%20%28double-precision%29))
  (Variables|Default|SetHealth (Math|Float|Min(Float) (+ (Variables|Default|GetHealth) Heal%20Amount) (Variables|Default|GetMax%20Health)))
  (CallFunction|UpdateDisplayedHealth))

(fn PlayRemovalAnimation
  (Variables|Default|SetIs%20Being%20Removed true))

(fn TickRecentDamageAnimation
  (bind _health_bar (Variables|Default|GetHealth%20Bar))
  (bind _health_bar_2 (Variables|Default|GetHealth%20Bar))
  (bind _health_bar_3 (Variables|Default|GetHealth%20Bar))
  (bind _recentdamagebar (Variables|/Game/Night/UI_HealthBar.UI_HealthBar_C|GetRecentDamageBar _health_bar_2))
  (bind _recentdamagebar_2 (Variables|/Game/Night/UI_HealthBar.UI_HealthBar_C|GetRecentDamageBar _health_bar_3))
  (if (< (Variables|/Script/UMG.ProgressBar|GetPercent (Variables|/Game/Night/UI_HealthBar.UI_HealthBar_C|GetRecentDamageBar _health_bar)) (Variables|/Script/UMG.ProgressBar|GetPercent (Variables|/Game/Night/UI_HealthBar.UI_HealthBar_C|GetHealthBar _health_bar)))
    (Progress|SetPercent (Variables|/Game/Night/UI_HealthBar.UI_HealthBar_C|GetRecentDamageBar (Variables|Default|GetHealth%20Bar)) (Variables|/Script/UMG.ProgressBar|GetPercent (Variables|/Game/Night/UI_HealthBar.UI_HealthBar_C|GetHealthBar (Variables|Default|GetHealth%20Bar))))
    (else
      (Progress|SetPercent _recentdamagebar_2 (- (Variables|/Script/UMG.ProgressBar|GetPercent _recentdamagebar_2) (* (Utilities|Time|GetWorldDeltaSeconds) (Variables|Default|GetRecent%20Damage%20Anim%20Speed))))
      (Class|ProgressBar|SetFillColorandOpacity _recentdamagebar (Math|Color|Lerp(LinearColor) (Variables|Default|GetRecent%20Damage%20Anim%20Color%20Small%20Damage) (Variables|Default|GetRecent%20Damage%20Anim%20Color%20Huge%20Damage) (Math|Float|Clamp(Float) (/ (- (Variables|/Script/UMG.ProgressBar|GetPercent _recentdamagebar) (Variables|/Script/UMG.ProgressBar|GetPercent (Variables|/Game/Night/UI_HealthBar.UI_HealthBar_C|GetHealthBar (Variables|Default|GetHealth%20Bar)))) (Variables|Default|GetRecent%20Damage%20Anim%20Color%20Threshold))))))))

(fn TickRemovalAnimation
  (bind _health_bar (Variables|Default|GetHealth%20Bar))
  (Widget|SetRenderOpacity _health_bar (- (Class|Widget|GetRenderOpacity _health_bar) (* (Utilities|Time|GetWorldDeltaSeconds) (Variables|Default|GetRemoval%20Anim%20Speed)))))