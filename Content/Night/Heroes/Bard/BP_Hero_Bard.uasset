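; BP_Hero_Bard is the Bard hero, whose Lute and Harp weapon components slow the enemies they hit.
; On BeginPlay it binds both weapons' hit events to one handler that adds a stacking, timed negative status effect, tagged with the ability name, to the enemy.
; LoadLibData fills the slow amount, duration and stack cap from the hero's library data, and each new hit resets all effects with the same tag.
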(event Custom|Event%20Weapon%20Hit%20Enemy
  (params (Weapon :type BPC%20Weapon%20Object%20Reference) (Enemy :type BP%20Enemy%20Object%20Reference) (Damage%20Amount :type Float%20%28double-precision%29) (Knockback%20Vec :type Vector))
  (Default|AddStatusEffect (Variables|/Game/Night/Enemies/BP_Enemy.BP_Enemy_C|GetBPC_StatusEffectController Enemy) (Utilities|Struct|MakeF_StatusEffect (.AbilityName (Utilities|Struct|BreakF_Hero_Lib (Variables|Default|GetLib%20Data))) "NewEnumerator0" (* (Variables|Hero|Bard|GetSlow%20%25) -1.0) (Variables|Hero|Bard|GetSlow%20Duration) 0) (Variables|Hero|Bard|GetSlow%20Max%20Stacks) true))

(event EventBeginPlay
  (|CallParentFunction)
  (Utilities|FlowControl|Sequence
    (:then_0
      (EventDispatchers|BindEventtoOnWeaponHitEnemy (Variables|Default|GetBPC_Weapon_Lute) (delegate Custom|Event%20Weapon%20Hit%20Enemy)))
    (:then_1
      (EventDispatchers|BindEventtoOnWeaponHitEnemy (Variables|Default|GetBPC_Weapon_Harp) (delegate Custom|Event%20Weapon%20Hit%20Enemy)))))

(event Collision|EventActorBeginOverlap
  (params (OtherActor :type Actor%20Object%20Reference)))

(event EventTick
  (params (DeltaSeconds :type Float%20%28single-precision%29)))

(fn ConstructionScript
  (|CallParentFunction))

(fn LoadLibData
  (bind _lib_data (Variables|Default|GetLib%20Data))
  (bind (_unlocktype _weapon1 _weapon2 _abilityname _abilitydescription _moveenhancementname _moveenhancementdescription _basehealth _basemovespeed _attr1 _val1 _attr2 _val2 _attr3 _val3) (Utilities|Struct|BreakF_Hero_Lib _lib_data))
  (|CallParentFunction)
  (Utilities|FlowControl|Sequence
    (:then_0
      (Variables|Hero|Bard|SetSlow%20Max%20Stacks (Math|Float|Truncate _val1)))
    (:then_1
      (Variables|Hero|Bard|SetSlow%20%25 _val2))
    (:then_2
      (Variables|Hero|Bard|SetSlow%20Duration _val3))))