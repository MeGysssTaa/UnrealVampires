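; BP_Hero is a hero character for the Night part of the game, configured from the DT_Heroes data table row matching its Name.
; On BeginPlay it applies base health to BPCDamageable and base move speed to CharacterMovement, printing an error if the row is missing.
; Min analog walk speed equals max walk speed, keeping movement speed constant.
; It also tints the component's health bar widget green, then adds the UI_Night widget to the viewport.
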(event EventBeginPlay
  (Utilities|FlowControl|Sequence
    (:then_0
      (CallFunction|LoadLibData))
    (:then_1
      (bind _asui_health_bar (Utilities|Casting|CastToUI_HealthBar (UserInterface|GetWidget (Variables|/Game/Night/BP_Damageable_Actor.BP_Damageable_Actor_C|GetWidget (Variables|/Game/Night/BPC_Damageable.BPC_Damageable_C|GetHealth%20Bar%20Holder%20Actor (Variables|Default|GetBPC_Damageable))))))
      (Class|ProgressBar|SetFillColorandOpacity (Variables|/Game/Night/UI_HealthBar.UI_HealthBar_C|GetHealthBar _asui_health_bar) "(R=0.000000,G=1.000000,B=0.207111,A=1.000000)"))
    (:then_2
      (bind _returnvalue (UserInterface|CreateWidget "/Game/Night/UI_Night.UI_Night_C"))
      (UserInterface|Viewport|AddtoViewport _returnvalue 0))))

(fn ConstructionScript)

(fn LoadLibData
  (bind _returnvalue (Utilities|GetDataTableRow "/Game/Night/Heroes/DT_Heroes.DT_Heroes" (Variables|Hero|GetName))
    (:then
      (bind _output_get (Variables|Hero|SetLib%20Data _returnvalue))
      (Utilities|FlowControl|Sequence
        (:then_0
          (Default|SetMaxHealth (Variables|Default|GetBPC_Damageable) (.BaseHealth (Utilities|Struct|BreakF_Hero_Lib _output_get)) true))
        (:then_1
          (CallFunction|SetConstMoveSpeed (.BaseMoveSpeed (Utilities|Struct|BreakF_Hero_Lib _output_get))))))
    (:RowNotFound
      (Development|PrintString (Utilities|String|Append "ERROR: Hero could not be found in data table by its 'Name'! Skipping 'Load Lib Data'." " --- " (Utilities|GetDisplayName self) " --- " (Utilities|String|ToString(Name) (Variables|Hero|GetName))) true true "(R=1.000000,G=0.058333,B=0.058333,A=1.000000)" 6e+01))))

(fn SetConstMoveSpeed
  (params (Move%20Speed :type Float%20%28double-precision%29))
  (bind _charactermovement (Variables|Character|GetCharacterMovement))
  (bind _output_get (Variables|/Script/Engine.CharacterMovementComponent|SetMaxWalkSpeed _charactermovement Move%20Speed))
  (Variables|/Script/Engine.CharacterMovementComponent|SetMinAnalogWalkSpeed _charactermovement _output_get))