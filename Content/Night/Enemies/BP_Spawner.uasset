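; BP_Spawner periodically spawns an actor at its own transform, serving as an enemy spawner for the Night game mode.
; A Tick countdown triggers each spawn and resets to the configured interval.
; Each spawn picks uniformly at random from Variants whose min/max level range contains the LevelState of the BP_Night actor found at BeginPlay.
; Spawning adjusts for collisions but always succeeds in placing the actor.
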(event EventBeginPlay
  (Utilities|FlowControl|Sequence
    (:then_0
      (Variables|Spawner|SetRem%20Seconds (Variables|Spawner|GetSpawn%20Interval%20Seconds)))
    (:then_1
      (bind _returnvalue (Actor|GetActorOfClass "/Game/Night/BP_Night.BP_Night_C"))
      (Variables|Spawner|SetNight _returnvalue))))

(event EventTick
  (params (DeltaSeconds :type Float%20%28single-precision%29))
  (bind _output_get (Variables|Spawner|SetRem%20Seconds (- (Variables|Spawner|GetRem%20Seconds) DeltaSeconds)))
  (if (<= _output_get 0.0)
    (Variables|Spawner|SetRem%20Seconds (Variables|Spawner|GetSpawn%20Interval%20Seconds))
    (CallFunction|Spawn)))

(fn ConstructionScript)

(fn Spawn
  (Game|SpawnActorfromClass (.SpawnedActor (Utilities|Struct|BreakSK_SpawnerEntry (.OutItem (Utilities|Array|Random (CallFunction|GetSpawnCandidates))))) (Transformation|GetActorTransform) "AdjustIfPossibleButAlwaysSpawn" 0 0))

(fn GetSpawnCandidates
  (for _array_element (Variables|Spawner|GetVariants)
    (if (CallFunction|IsValidSpawnCandidate _array_element)
      (Utilities|Array|Add (LocalVariables|GetLocal%20Candidates) _array_element)))
  (return (LocalVariables|GetLocal%20Candidates)))

(fn IsValidSpawnCandidate
  (params (Spawner%20Entry :type SK%20Spawner%20Entry%20Structure))
  (return (Math|Integer|InRange(Integer) (Variables|/Game/Night/BP_Night.BP_Night_C|GetLevel%20State (Variables|Spawner|GetNight)) (.minlevelstate Spawner%20Entry) (.maxlevelstate Spawner%20Entry))))