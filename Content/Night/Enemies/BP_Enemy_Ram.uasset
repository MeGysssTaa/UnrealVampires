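; Enemy for the Night part of the game that alternates between waiting and charging in a straight line.
; Tick runs a two-state machine: Idle counts down a preparation timer, then picks a destination from the Aiming mode, either the player's position or a random nearby navigable point.
; Ramming feeds that fixed direction into movement input for a random duration, without re-aiming, then returns to Idle.
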(event EventTick
  (params (DeltaSeconds :type Float%20%28single-precision%29))
  (|CallParentFunction DeltaSeconds)
  (switch Utilities|FlowControl|Switch|SwitchonE_Ram_State (Variables|Ram|GetRam%20State)
    (:NewEnumerator0
      (CallFunction|TickIdle))
    (:NewEnumerator2
      (CallFunction|TickRamming))))

(fn ConstructionScript
  (|CallParentFunction))

(fn GetNewRamDest
  (switch Utilities|FlowControl|Switch|SwitchonE_Ram_Aiming (Variables|Ram|GetAiming)
    (:NewEnumerator0
      (return (Transformation|GetActorLocation (Game|GetPlayerCharacter 0))))
    (:NewEnumerator1
      (bind _randomlocation (Class|NavigationSystemV1|GetRandomLocationinNavigableRadius (Transformation|GetActorLocation) 1e+02 0 0))
      (return _randomlocation))))

(fn TickIdle
  (if (> (Variables|Ram|GetRem%20Idle%20Time) 0.0)
    (Variables|Ram|SetRem%20Idle%20Time (- (Variables|Ram|GetRem%20Idle%20Time) (Utilities|Time|GetWorldDeltaSeconds)))
    (else
      (CallFunction|BeginRamming))))

(fn BeginRamming
  (Variables|Ram|SetRam%20Dir (- (CallFunction|GetNewRamDest) (Transformation|GetActorLocation)))
  (Variables|Ram|SetRem%20Ram%20Time (Math|Random|RandomFloatinRange (Variables|Ram|GetMin%20Ram%20Seconds) (Variables|Ram|GetMax%20Ram%20Seconds)))
  (Variables|Ram|SetRam%20State "NewEnumerator2")
  (CallFunction|TickRamming))

(fn TickRamming
  (if (> (Variables|Ram|GetRem%20Ram%20Time) 0.0)
    (Pawn|Input|AddMovementInput (Variables|Ram|GetRam%20Dir) 1.0 false)
    (Variables|Ram|SetRem%20Ram%20Time (- (Variables|Ram|GetRem%20Ram%20Time) (Utilities|Time|GetWorldDeltaSeconds)))
    (else
      (Variables|Ram|SetRam%20Dir "0, 0, 0")
      (Variables|Ram|SetRem%20Idle%20Time (Variables|Ram|GetPrepare%20Seconds))
      (Variables|Ram|SetRam%20State "NewEnumerator0"))))