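; Base enemy character for the Night mode that loads health, speed, damage, knockback resistance and gold from DT_Enemies by its Name.
; It damages the hero on capsule contact with a cooldown, plays random voice lines and per-surface footsteps, and scales speed through MoveSpeed attribute updates.
; KillEntity ragdolls it with an impulse, reports to BP_Night stats, splits gold into launched denomination coins and schedules cleanup.
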(event OnComponentHit(CapsuleComponent)
  (params (HitComponent :type Primitive%20Component%20Object%20Reference) (OtherActor :type Actor%20Object%20Reference) (OtherComp :type Primitive%20Component%20Object%20Reference) (NormalImpulse :type Vector :default "0, 0, 0") (Hit :type Hit%20Result%20Structure%20%28by%20ref%29))
  ;[0.136 0.8927 0.2749] Contact Damage
  (if (<= (Variables|Enemy|GetRem%20Attack%20Cooldown) 0.0)
    (bind _asbp_hero (Utilities|Casting|CastToBP_Hero OtherActor))
    (Default|Hurt (Variables|/Game/Night/Heroes/BP_Hero.BP_Hero_C|GetBPC_Damageable _asbp_hero) (.Damage (Utilities|Struct|BreakF_Enemy_Lib (Variables|Enemy|GetLib%20Data))) "0, 0, 0")
    (Variables|Enemy|SetRem%20Attack%20Cooldown 0.5)
    (Components|Activation|Activate (Variables|/Game/Night/Heroes/BP_Hero.BP_Hero_C|GetHurt%20Effect _asbp_hero) true)))

(event EventPlayFootstepSound
  (params (Location :type Vector :default "0, 0, 0") (Physical%20Surface%20Type :type EPhysicalSurface%20Enum :default "SurfaceType_Default"))
  (Audio|PlaySoundatLocation (.Value (Utilities|Map|Find (Variables|Enemy|GetFootstep%20Sounds) Physical%20Surface%20Type)) Location "0, 0, 0" 1.0 1.0 0.0 0 0 0 0))

(event EventKillEntity
  (params (Kill%20Impulse :type Vector :default "0, 0, 0"))
  ;[0.8844 0.4582 0.2644] Death
  (if (Actor|ActorHasTag "alive")
    (Utilities|FlowControl|Sequence
      (:then_0
        (Utilities|Array|RemoveItem (Variables|Actor|GetTags) "alive"))
      (:then_1
        (Physics|SetSimulatePhysics (Variables|Character|GetMesh) true)
        (Collision|SetCollisionEnabled (Variables|Character|GetMesh) "PhysicsOnly")
        (Collision|SetCollisionEnabled (Variables|Collision|GetCapsuleComponent) "PhysicsOnly"))
      (:then_2
        (Physics|AddImpulse (Variables|Character|GetMesh) Kill%20Impulse "None" false))
      (:then_3
        (CallFunction|DropGoldCoins (.Gold (Utilities|Struct|BreakF_Enemy_Lib (Variables|Enemy|GetLib%20Data))) (Variables|Enemy|GetCoin%20Denominations) (+ (Transformation|GetActorLocation) "0.000000,0.000000,100.000000") 0.0 (* Kill%20Impulse 0.0075) 1e+02))
      (:then_4
        (Default|PlayRemovalAnimation (Variables|Default|GetBPC_Damageable))
        (Utilities|FlowControl|Delay 1e+01)
        (bind _health_bar_holder_actor (Variables|/Game/Night/BPC_Damageable.BPC_Damageable_C|GetHealth%20Bar%20Holder%20Actor (Variables|Default|GetBPC_Damageable))
          (:then
            (Actor|DestroyActor _health_bar_holder_actor))
          (:else)))
      (:then_5
        (Default|StatsAdd (Variables|Enemy|GetNight%20) "EnemyKilled" 1.0))
      (:then_6
        (Utilities|FlowControl|Delay 3e+01)
        (Collision|SetCollisionResponsetoAllChannels (Variables|Character|GetMesh) "ECR_Ignore")
        (Actor|SetLifeSpan 5.0))
      (:then_7
        (Audio|PlaySoundatLocation (Variables|Enemy|GetDeath%20Sound) (Transformation|GetActorLocation) "0, 0, 0" 1.0 1.0 0.0 0 0 0 0)))))

(event EventTick
  (params (DeltaSeconds :type Float%20%28single-precision%29))
  (Utilities|FlowControl|Sequence
    (:then_0
      (Variables|Enemy|SetRem%20Attack%20Cooldown (- (Variables|Enemy|GetRem%20Attack%20Cooldown) (Utilities|Time|GetWorldDeltaSeconds))))
    (:then_1
      (if (Actor|ActorHasTag "alive")
        (bind _output_get (Variables|Enemy|SetRem%20Speak%20Cooldown (- (Variables|Enemy|GetRem%20Speak%20Cooldown) (Utilities|Time|GetWorldDeltaSeconds))))
        (if (<= _output_get 0.0)
          (Variables|Enemy|SetRem%20Speak%20Cooldown (Math|Random|RandomFloatinRange (Variables|Enemy|GetMin%20Rand%20Speak%20Delay%20Seconds) (Variables|Enemy|GetMax%20Rand%20Speak%20Delay%20Seconds)))
          (Audio|PlaySoundatLocation (Variables|Enemy|GetSpeak%20Sound) (Transformation|GetActorLocation) "0, 0, 0" 1.0 1.0 0.0 0 0 0 0))))))

(event EventUpdateEntityAttribute(MoveSpeed)
  (params (New%20Base%20Multiplier :type Float%20%28double-precision%29))
  (CallFunction|SetFixedMoveSpeed (* New%20Base%20Multiplier (.MoveSpeed (Utilities|Struct|BreakF_Enemy_Lib (Variables|Enemy|GetLib%20Data))))))

(event EventBeginPlay
  ;[0.6217 0.3875 0.9052] Common Setup / Initialization
  (Utilities|FlowControl|Sequence
    (:then_0
      (bind _returnvalue (Actor|GetActorOfClass "/Game/Night/BP_Night.BP_Night_C"))
      (Variables|Enemy|SetNight%20 _returnvalue)
      (Default|StatsAdd (Variables|Enemy|GetNight%20) "EnemySpawn" 1.0)
      (Utilities|Array|AddUnique (Variables|Actor|GetTags) "alive"))
    (:then_1
      (CallFunction|LoadLibData))
    (:then_2
      (Variables|Enemy|SetRem%20Speak%20Cooldown (Math|Random|RandomFloatinRange (Variables|Enemy|GetMin%20Rand%20Speak%20Delay%20Seconds) (Variables|Enemy|GetMax%20Rand%20Speak%20Delay%20Seconds))))))

(fn ConstructionScript)

(fn LoadLibData
  (bind _returnvalue (Utilities|GetDataTableRow "/Game/Night/Enemies/DT_Enemies.DT_Enemies" (Variables|Enemy|GetName))
    (:then
      (bind _output_get (Variables|Enemy|SetLib%20Data _returnvalue))
      (Utilities|FlowControl|Sequence
        (:then_0
          (Default|SetMaxHealth (Variables|Default|GetBPC_Damageable) (.Health (Utilities|Struct|BreakF_Enemy_Lib _output_get)) true))
        (:then_1
          (CallFunction|SetFixedMoveSpeed (.MoveSpeed (Utilities|Struct|BreakF_Enemy_Lib _output_get))))
        (:then_2
          (Variables|/Game/Night/BPC_Knockbackable.BPC_Knockbackable_C|SetKnockback%20Resistence%20%25 (Variables|Default|GetBPC_Knockbackable) (.KnockbackResistence (Utilities|Struct|BreakF_Enemy_Lib _output_get))))))
    (:RowNotFound
      (Development|PrintString (Utilities|String|Append "ERROR: Enemy could not be found in data table by its 'Name'! Skipping 'Load Lib Data'." " --- " (Utilities|GetDisplayName self) " --- " (Utilities|String|ToString(Name) (Variables|Enemy|GetName))) true true "(R=1.000000,G=0.058333,B=0.058333,A=1.000000)" 6e+01))))

(fn SetFixedMoveSpeed
  (params (Move%20Speed :type Float%20%28double-precision%29))
  (bind _charactermovement (Variables|Character|GetCharacterMovement))
  (bind _output_get (Variables|/Script/Engine.CharacterMovementComponent|SetMaxWalkSpeed _charactermovement Move%20Speed))
  (Variables|/Script/Engine.CharacterMovementComponent|SetMinAnalogWalkSpeed _charactermovement _output_get))

(fn DropGoldCoins
  (params (Gold%20Amount :type Integer) (Coin%20Denominations :type Array%20of%20Integers) (Base%20Location :type Vector) (Random%20Location%20Offset%20Amplitude%20XY :type Float%20%28double-precision%29) (Base%20Velocity :type Vector) (Random%20Velocity%20Offset%20Amplitude%20XY :type Float%20%28double-precision%29))
  (bind _returnvalue (* Random%20Location%20Offset%20Amplitude%20XY -1.0))
  (bind _returnvalue_2 (* Random%20Velocity%20Offset%20Amplitude%20XY -1.0))
  (if (>= Gold%20Amount 0)
    (LocalVariables|SetLocal%20Remaining%20Gold Gold%20Amount)
    (for _array_element Coin%20Denominations
      (LocalVariables|SetLocal%20%28For%29%20Coins%20Of%20This%20Denom (/ (LocalVariables|GetLocal%20Remaining%20Gold) _array_element))
      (LocalVariables|SetLocal%20Remaining%20Gold (- (LocalVariables|GetLocal%20Remaining%20Gold) (* (LocalVariables|GetLocal%20%28For%29%20Coins%20Of%20This%20Denom) _array_element)))
      (for _index (range 1 (LocalVariables|GetLocal%20%28For%29%20Coins%20Of%20This%20Denom))
        (bind _returnvalue_3 (Game|SpawnActorfromClass "/Game/Economy/BP_PickableCoin.BP_PickableCoin_C" (Math|Transform|MakeTransform (+ Base%20Location (Math|Vector|MakeVector (Math|Random|RandomFloatinRange _returnvalue Random%20Location%20Offset%20Amplitude%20XY) (Math|Random|RandomFloatinRange _returnvalue Random%20Location%20Offset%20Amplitude%20XY) 0.0)) "0, 0, 0" "1.000000,1.000000,1.000000") "AlwaysSpawn" 0 _array_element 0))
        (Character|LaunchCharacter _returnvalue_3 (+ Base%20Velocity (Math|Vector|MakeVector (Math|Random|RandomFloatinRange _returnvalue_2 Random%20Velocity%20Offset%20Amplitude%20XY) (Math|Random|RandomFloatinRange _returnvalue_2 Random%20Velocity%20Offset%20Amplitude%20XY) 6e+02)) false false))
      (LocalVariables|SetLocal%20%28For%29%20Coins%20Of%20This%20Denom 0))))