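; BP_Night is an actor for the night phase that tracks session stats and holds the game-end logic.
; BeginPlay caches the Undeads game instance and shows the night cheats widget, while Tick accumulates GameTime in a Stats map through get/set/add helpers.
; The end branch shows UI_GameEnd, stops ticking and kills living enemies, but its condition is hardwired false.
; Time and kill-count checks and low-population enemy spawning remain unconnected.
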(event EventBeginPlay
  (bind _asgi_undeads (Utilities|Casting|CastToGI_Undeads (Game|GetGameInstance)))
  (Variables|Default|SetMy%20Game%20Instance _asgi_undeads)
  (bind _returnvalue (UserInterface|CreateWidget "/Game/Night/UI_Night_Cheats.UI_Night_Cheats_C"))
  (UserInterface|Viewport|AddtoViewport _returnvalue 0))

(event EventTick
  (params (DeltaSeconds :type Float%20%28single-precision%29))
  (CallFunction|StatsAdd "GameTime" (Utilities|Time|GetWorldDeltaSeconds))
  (if (or false false)
    (bind _returnvalue (UserInterface|CreateWidget "/Game/Night/UI_GameEnd.UI_GameEnd_C"))
    (UserInterface|Viewport|AddtoViewport _returnvalue 0)
    (Actor|Tick|SetActorTickEnabled false)
    (bind _outactors (Actor|GetAllActorsOfClasswithTag "/Game/Night/Enemies/BP_Enemy.BP_Enemy_C" "alive"))
    (Default|KillEntity _outactors "0, 0, 0")))

(fn ConstructionScript)

(fn GetEnemies
  (bind _outactors (Actor|GetAllActorsOfClass "/Game/Night/Enemies/BP_Enemy.BP_Enemy_C"))
  (return _outactors))

(fn StatsAdd
  (params (Attr :type String) (Val :type Float%20%28double-precision%29))
  (Utilities|Map|Add (Variables|Default|GetStats) Attr (+ (.Value (Utilities|Map|Find (Variables|Default|GetStats) Attr)) Val)))

(fn StatsGet
  (params (Attr :type String))
  (return (.Value (Utilities|Map|Find (Variables|Default|GetStats) Attr))))

(fn StatsSet
  (params (Attr :type String) (Val :type Float%20%28double-precision%29))
  (Utilities|Map|Add (Variables|Default|GetStats) Attr Val))