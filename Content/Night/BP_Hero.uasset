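; BP_Hero is the player hero Blueprint for the Night portion of the game.
; On BeginPlay it tints the health bar from its damageable component's widget green and adds the UI_Night widget to the viewport.
; AddWeapon looks up a tag as a row name in the DT_Weapons data table and attaches that row's component class to the hero.
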(event EventBeginPlay
  (bind _asui_health_bar (Utilities|Casting|CastToUI_HealthBar (UserInterface|GetWidget (Variables|/Game/Night/BP_Damageable_Actor.BP_Damageable_Actor_C|GetWidget (Variables|/Game/Night/BPC_Damageable.BPC_Damageable_C|GetHealth%20Bar%20Holder%20Actor (Variables|Default|GetBPC_Damageable))))))
  (Class|ProgressBar|SetFillColorandOpacity (Variables|/Game/Night/UI_HealthBar.UI_HealthBar_C|GetHealthBar _asui_health_bar) "(R=0.000000,G=1.000000,B=0.207111,A=1.000000)")
  (bind _returnvalue (UserInterface|CreateWidget "/Game/Night/UI_Night.UI_Night_C"))
  (UserInterface|Viewport|AddtoViewport _returnvalue 0))

(fn ConstructionScript)

(fn AddWeapon
  (params (Tag :type String))
  (bind _returnvalue (Utilities|GetDataTableRow "/Game/Night/Weapons/DT_Weapons.DT_Weapons" (Utilities|String|StringToName Tag))
    (:then
      (Game|AddComponentbyClass (.Component (Utilities|Struct|BreakSK_Weapon _returnvalue))))))