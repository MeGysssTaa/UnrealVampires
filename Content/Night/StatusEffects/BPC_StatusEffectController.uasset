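; Actor component that tracks timed status effects on its owner and turns them into a move speed multiplier.
; A map holds each effect's remaining seconds, counted down every Tick, with functions to add, clear or reset durations by tag.
; Adding, clearing or expiry combines one attribute's percentage changes multiplicatively and messages the owner with the result.
; An additive combiner is also defined but not called here.
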(event EventBeginPlay)

(event EventTick
  (params (DeltaSeconds :type Float%20%28single-precision%29))
  (CallFunction|TickStatusEffects))

(fn AddStatusEffect
  (params (Status%20Effect :type F%20Status%20Effect%20Structure))
  (Utilities|Map|Add (Variables|Default|GetActive%20Effects) Status%20Effect (.DurationSeconds (Utilities|Struct|BreakF_StatusEffect Status%20Effect)))
  (CallFunction|UpdateStatusEffects))

(fn ClearStatusEffects
  (Utilities|Map|Clear (Variables|Default|GetActive%20Effects))
  (CallFunction|UpdateStatusEffects))

(fn ResetDurationsforTag
  (params (Status%20Effects%20Tag :type Name :default "Generic"))
  (bind _keys (Utilities|Map|Keys (Variables|Default|GetActive%20Effects)))
  (for _array_element _keys
    (if (== (.Tag (Utilities|Struct|BreakF_StatusEffect _array_element)) Status%20Effects%20Tag)
      (Utilities|Map|Add (Variables|Default|GetActive%20Effects) _array_element (.DurationSeconds (Utilities|Struct|BreakF_StatusEffect _array_element))))))

(fn TickStatusEffects
  (bind _keys (Utilities|Map|Keys (Variables|Default|GetActive%20Effects)))
  (for _array_element _keys
    (if (> (- (.Value (Utilities|Map|Find (Variables|Default|GetActive%20Effects) _array_element)) (Utilities|Time|GetWorldDeltaSeconds)) 0.0)
      (Utilities|Map|Add (Variables|Default|GetActive%20Effects) _array_element (- (.Value (Utilities|Map|Find (Variables|Default|GetActive%20Effects) _array_element)) (Utilities|Time|GetWorldDeltaSeconds)))
      (else
        (Utilities|Array|Add (LocalVariables|GetLocal%20Expired%20Effects) _array_element))))
  (for _array_element_2 (LocalVariables|GetLocal%20Expired%20Effects)
    (Utilities|Map|Remove (Variables|Default|GetActive%20Effects) _array_element_2))
  (if (Utilities|Array|IsNotEmpty (LocalVariables|GetLocal%20Expired%20Effects))
    (CallFunction|UpdateStatusEffects)))

(fn UpdateStatusEffects
  (Utilities|FlowControl|Sequence
    (:then_0
      (Class|BPIAttributableEntity|UpdateEntityAttribute(MoveSpeed)(Message) (Components|GetOwner) (CallFunction|GetMultiplicativeMultiplier (CallFunction|GetEffectsbyAttribute "NewEnumerator0"))))))

(fn GetEffectsbyAttribute
  (params (Entity%20Attribute :type E_EntityAttribute%20Enum :default "NewEnumerator0"))
  (bind _keys (Utilities|Map|Keys (Variables|Default|GetActive%20Effects)))
  (for _array_element _keys
    (if (Utilities|Enum|Equal(Enum) (.Attribute (Utilities|Struct|BreakF_StatusEffect _array_element)) Entity%20Attribute)
      (Utilities|Array|Add (LocalVariables|GetLocal%20Result) _array_element)))
  (return (LocalVariables|GetLocal%20Result)))

(fn GetAdditiveMultiplier
  (params (Status%20Effects :type Array%20of%20F%20Status%20Effect%20Structures))
  (for _array_element Status%20Effects
    (LocalVariables|SetLocal%20Multiplier (+ (LocalVariables|GetLocal%20Multiplier) (/ (.Change (Utilities|Struct|BreakF_StatusEffect _array_element)) 1e+02))))
  (return (LocalVariables|GetLocal%20Multiplier)))

(fn GetMultiplicativeMultiplier
  (params (Status%20Effects :type Array%20of%20F%20Status%20Effect%20Structures))
  (for _array_element Status%20Effects
    (LocalVariables|SetLocal%20Multiplier (* (+ (/ (.Change (Utilities|Struct|BreakF_StatusEffect _array_element)) 1e+02) 1.0) (LocalVariables|GetLocal%20Multiplier))))
  (return (LocalVariables|GetLocal%20Multiplier)))