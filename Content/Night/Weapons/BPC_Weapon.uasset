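; BPC_Weapon is a base weapon component that fires automatically on a cooldown and tags itself at BeginPlay.
; Tick counts down the cooldown, then resets it and calls an empty Attack function, apparently meant for child weapons to override.
; Shared helpers find the nearest or a random BP_Enemy and apply damage with horizontal knockback away from the owner through the enemy's damageable and knockback components.
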(event EventBeginPlay
  (Utilities|Array|Add (Variables|Default|GetComponentTags) (Utilities|String|StringToName (Variables|Weapon|GetTag))))

(event EventTick
  (params (DeltaSeconds :type Float%20%28single-precision%29))
  (if (> (Variables|Weapon|GetCooldown) 0.0)
    (Variables|Weapon|SetCooldown (- (Variables|Weapon|GetCooldown) (Utilities|Time|GetWorldDeltaSeconds)))
    (else
      (Variables|Weapon|SetCooldown (Variables|Weapon|GetCooldown%20Max))
      (CallFunction|Attack))))

(fn DamageEnemy
  (params (Enemy :type BP%20Enemy%20Object%20Reference))
  (LocalVariables|SetLocal%20Knockback%20Vec (* (Math|Vector|Normalize (- (Math|Conversions|ToVector2D(Vector) (Transformation|GetActorLocation Enemy)) (Math|Conversions|ToVector2D(Vector) (Transformation|GetActorLocation (Components|GetOwner))))) (Variables|Weapon|GetKnockback)))
  (Default|Hurt (Variables|/Game/Night/BP_Enemy.BP_Enemy_C|GetBPC_Damageable Enemy) (Variables|Weapon|GetDamage) (* (LocalVariables|GetLocal%20Knockback%20Vec) 15.0))
  (Default|KnockBack (Variables|/Game/Night/BP_Enemy.BP_Enemy_C|GetBPC_Knockbackable Enemy) (LocalVariables|GetLocal%20Knockback%20Vec)))

(fn Attack)

(fn GetNearestEnemy
  (params (In%20Location :type Vector))
  (bind _outactors (Actor|GetAllActorsOfClass "/Game/Night/BP_Enemy.BP_Enemy_C"))
  (bind _asbp_enemy (Utilities|Casting|CastToBP_Enemy (.ReturnValue (Actor|FindNearestActor In%20Location _outactors))))
  (return _asbp_enemy))

(fn GetRandomEnemy
  (bind _outactors (Actor|GetAllActorsOfClass "/Game/Night/BP_Enemy.BP_Enemy_C"))
  (return (.OutItem (Utilities|Array|Random _outactors))))