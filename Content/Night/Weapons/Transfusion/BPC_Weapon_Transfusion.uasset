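; Transfusion weapon component that heals its owner from library data, built to hit the nearest enemy in range in a life-drain attack.
; Tick feeds the owner's location to each tracked Niagara system as its force origin, pulling effects toward the owner.
; The attack logic (hit, heal, spawn and track effect, report cooldown) is disconnected from the Attack entry, so as written Attack does nothing.
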(event EventBeginPlay
  (|CallParentFunction)
  (Variables|Weapon|SetOwner%20Damageable (Actor|GetComponentbyClass (Components|GetOwner) "/Game/Night/BPC_Damageable.BPC_Damageable_C")))

(event EventTick
  (params (DeltaSeconds :type Float%20%28single-precision%29))
  (|CallParentFunction DeltaSeconds)
  (for _array_element (Variables|Default|GetParticle%20Systems)
    (Niagara|SetNiagaraVariable(Vector3) _array_element "Force Origin" (Transformation|GetActorLocation (Components|GetOwner)))))

(fn Attack)

(fn LoadLibData
  (|CallParentFunction)
  (Variables|Weapon|SetHeal (.Val1 (Utilities|Struct|BreakF_Weapon_Lib (Variables|Default|GetLib%20Data)))))

(fn UnregisterParticleSystem
  (params (PSystem :type Niagara%20Component%20Object%20Reference))
  (Utilities|Array|RemoveItem (Variables|Default|GetParticle%20Systems) PSystem))