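; Stab weapon component that damages every enemy in a line in front of its owner.
; Attack sweeps a multi-object capsule trace for Pawns along the owner's forward vector, with Range setting length and half of AOE the radius.
; BP_Enemy hits are gathered uniquely into LocalEnemies, then each goes to DamageEnemy, avoiding duplicate damage.
; The trace's debug drawing is left on.
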(event EventBeginPlay)

(event EventTick
  (params (DeltaSeconds :type Float%20%28single-precision%29))
  (|CallParentFunction DeltaSeconds) ; This node is disabled and will not be called.\nDrag off pins to build functionality.
)

(fn Attack
  (bind _returnvalue (Components|GetOwner))
  (bind _returnvalue_2 (Transformation|GetActorLocation _returnvalue))
  (bind _outhits (Class|KismetSystemLibrary|CapsuleTraceMultiforObjects _returnvalue_2 (+ _returnvalue_2 (* (Transformation|GetActorForwardVector _returnvalue) (Variables|Default|GetRange))) (/ (Variables|Default|GetAOE) 2.0) 2e+02 (Utilities|Array|MakeArray "ObjectTypeQuery3") false 0 "ForDuration" true "(R=0.023681,G=0.975000,B=0.803285,A=1.000000)" "(R=0.000000,G=1.000000,B=0.000000,A=1.000000)" 0.5))
  (for _array_element _outhits
    (bind _asbp_enemy (Utilities|Casting|CastToBP_Enemy (.HitActor (Collision|BreakHitResult _array_element))))
    (Utilities|Array|AddUnique (LocalVariables|GetLocal%20Enemies) _asbp_enemy))
  (for _array_element_2 (LocalVariables|GetLocal%20Enemies)
    (CallFunction|DamageEnemy _array_element_2)))