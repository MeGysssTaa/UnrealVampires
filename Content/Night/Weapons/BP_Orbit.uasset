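; BP_Orbit is a weapon-folder Blueprint that keeps registered "Sputnik" actors circling its own location.
; Actors join through AddSputnik, and Tick removes invalid entries by iterating the array in reverse.
; Each Tick advances a shared angle at constant speed and spaces the remaining actors evenly on a horizontal circle of Radius.
; Actors ease toward their slots with a fixed-alpha, per-frame lerp, so gaps close smoothly when the count changes.
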(event EventBeginPlay)

(event EventTick
  (params (DeltaSeconds :type Float%20%28single-precision%29))
  (Variables|Default|SetDelta (+ (Variables|Default|GetDelta) (* (Utilities|Time|GetWorldDeltaSeconds) -2.0)))
  (Utilities|FlowControl|Sequence
    (:then_0
      (bind (_arrayindex _arrayelement) (Utilities|Array|ReverseforEachLoop (Variables|Default|GetSputniks))
        (:LoopBody
          (Utilities|IsValid _arrayelement
            (:Is%20Not%20Valid
              (Utilities|Array|RemoveIndex (Variables|Default|GetSputniks) _arrayindex))))))
    (:then_1
      (Variables|Default|SetLength (Utilities|Array|Length (Variables|Default|GetSputniks)))
      (for (_array_element _array_index) (Variables|Default|GetSputniks)
        (Transformation|SetActorLocation _array_element (Math|Vector|Lerp(Vector) (Transformation|GetActorLocation _array_element) (+ (Transformation|GetActorLocation) (Math|Vector|MakeVector (* (Variables|Default|GetRadius) (Math|Trig|Sin(Radians) (+ (* (/ (Math|Conversions|ToFloat(Integer) _array_index) (Variables|Default|GetLength)) (Math|Trig|GetPI) 2.0) (Variables|Default|GetDelta)))) (* (Math|Trig|Cos(Radians) (+ (* (/ (Math|Conversions|ToFloat(Integer) _array_index) (Variables|Default|GetLength)) (Math|Trig|GetPI) 2.0) (Variables|Default|GetDelta))) (Variables|Default|GetRadius)) 0.0)) 0.1) false false)))))

(fn ConstructionScript)

(fn AddSputnik
  (params (Actor :type Actor%20Object%20Reference))
  (Utilities|Array|Add (Variables|Default|GetSputniks) Actor))