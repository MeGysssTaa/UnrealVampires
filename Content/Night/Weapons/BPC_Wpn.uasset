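; Base weapon component for the Night part of the game that attacks automatically on a repeating cooldown.
; Tick counts the cooldown down, then resets it and calls Attack, which is empty here.
; StrikeEnemy applies damage through the enemy's Damageable component and pushes it away from the owner through its Knockbackable component, using a normalized 2D direction scaled by Knockback.
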(event EventTick
  (params (DeltaSeconds :type Float%20%28single-precision%29))
  (if (> (Variables|Default|GetCooldown) 0.0)
    (Variables|Default|SetCooldown (- (Variables|Default|GetCooldown) (Utilities|Time|GetWorldDeltaSeconds)))
    (else
      (Variables|Default|SetCooldown (Variables|Default|GetCooldown%20Max))
      (CallFunction|Attack))))

(fn StrikeEnemy
  (params (Enemy :type BP%20Enemy%20Object%20Reference))
  (Default|Hurt (Variables|/Game/Night/Enemies/BP_Enemy.BP_Enemy_C|GetBPC_Damageable Enemy) (Variables|Default|GetDamage))
  (Default|KnockBack (Variables|/Game/Night/Enemies/BP_Enemy.BP_Enemy_C|GetBPC_Knockbackable Enemy) (* (Math|Vector|Normalize (- (Math|Conversions|ToVector2D(Vector) (Transformation|GetActorLocation Enemy)) (Math|Conversions|ToVector2D(Vector) (Transformation|GetActorLocation (Components|GetOwner))))) (Variables|Default|GetKnockback))))

(fn Attack)