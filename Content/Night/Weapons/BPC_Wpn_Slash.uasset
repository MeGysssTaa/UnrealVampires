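; BPC_Wpn_Slash is a weapon component that performs a cone-shaped slash attack around its owner.
; Attack gathers BP_Enemy pawns with a sphere overlap of radius Range, drawing a brief debug sphere.
; It keeps those whose angle from the owner's forward vector is under half of AOE, treating AOE as arc width in degrees, and calls StrikeEnemy on each.
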(event EventBeginPlay)

(event EventTick
  (params (DeltaSeconds :type Float%20%28single-precision%29))
  (|CallParentFunction DeltaSeconds) ; This node is disabled and will not be called.\nDrag off pins to build functionality.
)

(fn Attack
  (bind _returnvalue (Components|GetOwner))
  (bind _range (Variables|Default|GetRange))
  (bind _returnvalue_2 (Transformation|GetActorLocation _returnvalue))
  ;[0.2029 0.2537 0.3052] Find enemies in range (sphere)
  (Rendering|Debug|DrawDebugSphere _returnvalue_2 _range 24 "(R=0.432638,G=0.153274,B=1.000000,A=1.000000)" 0.25 2.0)
  (bind _outactors (Collision|SphereOverlapActors _returnvalue_2 _range (Utilities|Array|MakeArray "ObjectTypeQuery3") "/Game/Night/Enemies/BP_Enemy.BP_Enemy_C"))
  ;[0.2029 0.2537 0.3052] Find enemies within FOV/angle
  (for _array_element _outactors
    (if (< (Class|KismetMathLibrary|DegAcos (Math|Vector|DotProduct (Math|Vector|Normalize (- (Transformation|GetActorLocation _array_element) (Transformation|GetActorLocation (Components|GetOwner)))) (Transformation|GetActorForwardVector (Components|GetOwner)))) (/ (Variables|Default|GetAOE) 2.0))
      (bind _asbp_enemy (Utilities|Casting|CastToBP_Enemy _array_element))
      (CallFunction|StrikeEnemy _asbp_enemy))))