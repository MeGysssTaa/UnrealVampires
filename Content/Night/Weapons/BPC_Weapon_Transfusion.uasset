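; BPC_Weapon_Transfusion is a weapon component that damages the nearest enemy and heals its owner on each successful attack.
; On BeginPlay it caches the owner's BPC_Damageable component, and on loading library data it reads the heal amount from Val1.
; Attack searches for the nearest enemy within the library range, damages it, then heals the owner, doing neither when no target is found.
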(event EventBeginPlay
  (|CallParentFunction)
  (Variables|Weapon|SetOwner%20Damageable (Actor|GetComponentbyClass (Components|GetOwner) "/Game/Night/BPC_Damageable.BPC_Damageable_C")))

(event EventTick
  (params (DeltaSeconds :type Float%20%28single-precision%29))
  (|CallParentFunction DeltaSeconds) ; This node is disabled and will not be called.\nDrag off pins to build functionality.
)

(fn Attack
  (bind _returnvalue (Components|GetOwner))
  (bind _lib_data (Variables|Default|GetLib%20Data))
  (bind _range (Utilities|Struct|BreakF_Weapon_Lib _lib_data))
  (bind _returnvalue_2 (Transformation|GetActorLocation _returnvalue))
  (bind (_out_enemy _success) (CallFunction|GetNearestEnemy _returnvalue_2 _range))
  (|CallParentFunction)
  (if _success
    (CallFunction|DamageEnemy _out_enemy)
    (Default|Heal (Variables|Weapon|GetOwner%20Damageable) (Variables|Weapon|GetHeal))))

(fn LoadLibData
  (|CallParentFunction)
  (Variables|Weapon|SetHeal (.Val1 (Utilities|Struct|BreakF_Weapon_Lib (Variables|Default|GetLib%20Data)))))