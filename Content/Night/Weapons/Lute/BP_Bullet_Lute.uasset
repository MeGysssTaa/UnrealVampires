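; Projectile for the Lute weapon, layering lute-specific visuals onto the behavior of its parent bullet class.
; On hitting an enemy, it calls the parent logic, then spawns the lute hit Niagara system inactive at its location.
; It sets that effect's cone axis to the bullet's velocity before activating it, so the burst follows the travel direction.
; When destroyed, it deactivates its own Niagara effect.
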(event EventBeginPlay
  (|CallParentFunction))

(event Collision|EventActorBeginOverlap
  (params (OtherActor :type Actor%20Object%20Reference))
  (|CallParentFunction OtherActor) ; This node is disabled and will not be called.\nDrag off pins to build functionality.
)

(event EventTick
  (params (DeltaSeconds :type Float%20%28single-precision%29))
  (|CallParentFunction DeltaSeconds))

(event EventDestroyed
  (Components|Activation|Deactivate (Variables|Default|GetNiagara)))

(fn ConstructionScript
  (|CallParentFunction))

(fn OnBulletHitEnemy
  (params (Enemy :type BP%20Enemy%20Object%20Reference))
  (|CallParentFunction Enemy)
  (bind _returnvalue (Niagara|SpawnSystematLocation "/Game/Night/Weapons/Lute/FX_Weapon_Lute_Hit.FX_Weapon_Lute_Hit" (Transformation|GetActorLocation) "0, 0, 0" "1.000000,1.000000,1.000000" true false))
  (Niagara|SetNiagaraVariable(Vector3) _returnvalue "Cone Axis" (Transformation|GetVelocity))
  (Components|Activation|Activate _returnvalue false))