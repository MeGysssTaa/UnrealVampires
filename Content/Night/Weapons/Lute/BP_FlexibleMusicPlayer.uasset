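; Music player that cycles through a playlist, optionally shuffled at start, repeating each track a set number of times.
; Tick times the current track and steps the volume toward a target.
; Track changes and repeats crossfade on one audio component by fading out, swapping the sound, then fading back in.
; FadeToVolume can temporarily change volume, ignoring unforced requests until it begins returning to base volume.
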(event Custom|Fade%20To%20Volume
  (params (New%20Desired%20Volume :type Float%20%28double-precision%29) (Fade%20Speed :type Float%20%28double-precision%29) (Seconds%20Before%20Fading%20Back :type Float%20%28double-precision%29) (Force :type Boolean))
  (if (or (Variables|FlexibleMusicPlayer|GetAccepting%20Fade%20Requests) Force)
    (Variables|FlexibleMusicPlayer|SetDesired%20Volume New%20Desired%20Volume)
    (Variables|FlexibleMusicPlayer|SetCurrent%20Fade%20Speed Fade%20Speed)
    (if (> Seconds%20Before%20Fading%20Back 0.0)
      (Variables|FlexibleMusicPlayer|SetAccepting%20Fade%20Requests false)
      (Utilities|FlowControl|Delay Seconds%20Before%20Fading%20Back)
      (Variables|FlexibleMusicPlayer|SetAccepting%20Fade%20Requests true)
      (CallFunction|FadetoVolume (Variables|FlexibleMusicPlayer|GetBase%20Volume) (Variables|FlexibleMusicPlayer|GetCurrent%20Fade%20Speed) 0.0 false))))

(event Custom|Crossfade%20Into%20Track
  (params (New%20Track :type Sound%20Wave%20Object%20Reference))
  (CallFunction|FadetoVolume 0.0 (Variables|FlexibleMusicPlayer|GetCrossfade%20Speed) 0.0 true)
  (Utilities|FlowControl|Delay (Variables|FlexibleMusicPlayer|GetCrossfade%20Time))
  (Audio|Components|Audio|Stop (Variables|Default|GetAudio))
  (Audio|Components|Audio|SetSound (Variables|Default|GetAudio) New%20Track)
  (Audio|Components|Audio|Play (Variables|Default|GetAudio) 0.0)
  (CallFunction|FadetoVolume (Variables|FlexibleMusicPlayer|GetBase%20Volume) (Variables|FlexibleMusicPlayer|GetCrossfade%20Speed) 0.0 true))

(event EventBeginPlay
  (Utilities|FlowControl|Sequence
    (:then_0
      (Variables|FlexibleMusicPlayer|SetDesired%20Volume (Variables|FlexibleMusicPlayer|GetBase%20Volume)))
    (:then_1
      (Audio|Components|Audio|SetVolumeMultiplier (Variables|Default|GetAudio) (Variables|FlexibleMusicPlayer|GetBase%20Volume) :!class /Script/Engine.AudioComponent))
    (:then_2
      (if (Variables|FlexibleMusicPlayer|GetShuffle%20Tracks)
        (Utilities|Array|Shuffle (Variables|FlexibleMusicPlayer|GetTracks))))))

(event EventTick
  (params (DeltaSeconds :type Float%20%28single-precision%29))
  (CallFunction|UpdateTrack)
  (CallFunction|UpdateFadeVolume))

(fn ConstructionScript)

(fn UpdateFadeVolume
  (if (not (Math|Float|NearlyEqual(Float) (Variables|/Script/Engine.AudioComponent|GetVolumeMultiplier (Variables|Default|GetAudio)) (Variables|FlexibleMusicPlayer|GetDesired%20Volume) 0.01))
    (LocalVariables|SetLocal%20Volume%20Diff (* (Utilities|Time|GetWorldDeltaSeconds) (Variables|FlexibleMusicPlayer|GetCurrent%20Fade%20Speed)))
    (if (> (Variables|FlexibleMusicPlayer|GetDesired%20Volume) (Variables|/Script/Engine.AudioComponent|GetVolumeMultiplier (Variables|Default|GetAudio)))
      _
      (else
        (LocalVariables|SetLocal%20Volume%20Diff (* (LocalVariables|GetLocal%20Volume%20Diff) -1.0))))
    (Audio|Components|Audio|SetVolumeMultiplier (Variables|Default|GetAudio) (Math|Float|Clamp(Float) (+ (Variables|/Script/Engine.AudioComponent|GetVolumeMultiplier (Variables|Default|GetAudio)) (LocalVariables|GetLocal%20Volume%20Diff)) (Variables|FlexibleMusicPlayer|GetMin%20Volume) (Variables|FlexibleMusicPlayer|GetMax%20Volume)) :!class /Script/Engine.AudioComponent)))

(fn UpdateTrack
  ;[0.2605 0.4301 0.7594] Check if this is the first time we play after init
  (if (< (Variables|FlexibleMusicPlayer|GetCurrent%20Track%20Index) 0)
    ;[0 1 0.2054] Play next track (crossfade)
    (Variables|FlexibleMusicPlayer|SetCurrent%20Track%20Index (Math|Integer|%(Integer) (+ (Variables|FlexibleMusicPlayer|GetCurrent%20Track%20Index) 1) (Utilities|Array|Length (Variables|FlexibleMusicPlayer|GetTracks))) :!label _label)
    (Variables|FlexibleMusicPlayer|SetCurrent%20Track%20Loop%20Number 1)
    (Variables|FlexibleMusicPlayer|SetCurrent%20Track%20Loop%20Playing%20Time 0.0)
    (CallFunction|CrossfadeIntoTrack (.Track (Utilities|Struct|BreakF_FlexibleSoundPlayer_Track (Utilities|Array|Get(acopy) (Variables|FlexibleMusicPlayer|GetTracks) (Variables|FlexibleMusicPlayer|GetCurrent%20Track%20Index)))))
    (else
      (bind _output_get (Variables|FlexibleMusicPlayer|SetCurrent%20Track%20Loop%20Playing%20Time (+ (Variables|FlexibleMusicPlayer|GetCurrent%20Track%20Loop%20Playing%20Time) (Utilities|Time|GetWorldDeltaSeconds))))
      (if (>= _output_get (- (Variables|/Script/Engine.SoundBase|GetDuration (.Track (Utilities|Struct|BreakF_FlexibleSoundPlayer_Track (Utilities|Array|Get(acopy) (Variables|FlexibleMusicPlayer|GetTracks) (Variables|FlexibleMusicPlayer|GetCurrent%20Track%20Index))))) (Variables|FlexibleMusicPlayer|GetCrossfade%20Time)))
        (if (== (Variables|FlexibleMusicPlayer|GetCurrent%20Track%20Loop%20Number) (.LoopTimes (Utilities|Struct|BreakF_FlexibleSoundPlayer_Track (Utilities|Array|Get(acopy) (Variables|FlexibleMusicPlayer|GetTracks) (Variables|FlexibleMusicPlayer|GetCurrent%20Track%20Index)))))
          (goto _label)
          (else
            ;[1 0.7615 0.05719] Repeat current track (crossfade)
            (Variables|FlexibleMusicPlayer|SetCurrent%20Track%20Loop%20Playing%20Time 0.0)
            (Math|Integer|IncrementInt (Variables|FlexibleMusicPlayer|GetCurrent%20Track%20Loop%20Number)
              (:%20%20
                (CallFunction|CrossfadeIntoTrack (.Track (Utilities|Struct|BreakF_FlexibleSoundPlayer_Track (Utilities|Array|Get(acopy) (Variables|FlexibleMusicPlayer|GetTracks) (Variables|FlexibleMusicPlayer|GetCurrent%20Track%20Index)))))))))))))