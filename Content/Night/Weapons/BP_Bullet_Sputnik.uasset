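; BP_Bullet_Sputnik is a bullet variant that orbits as a satellite instead of flying as a projectile.
; On BeginPlay it runs the parent logic, then destroys its ProjectileMovement component so it no longer propels itself.
; It finds the BP_Orbit actor in the level and registers itself through AddSputnik, leaving any further handling to that actor.
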(event EventBeginPlay
  (|CallParentFunction)
  (Components|DestroyComponent (Variables|Default|GetProjectileMovement))
  (bind _returnvalue (Actor|GetActorOfClass "/Game/Night/Weapons/BP_Orbit.BP_Orbit_C"))
  (bind _output_get (Variables|Default|SetMy%20Orbit _returnvalue))
  (Default|AddSputnik _output_get self))

(event Collision|EventActorBeginOverlap
  (params (OtherActor :type Actor%20Object%20Reference)))

(event EventTick
  (params (DeltaSeconds :type Float%20%28single-precision%29)))

(fn ConstructionScript
  (|CallParentFunction))