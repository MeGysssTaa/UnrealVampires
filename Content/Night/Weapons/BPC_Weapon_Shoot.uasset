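; Weapon component that fires a projectile from its owner on each attack, passing it the pierce value and a reference to itself.
; Attack extends the parent and picks a spawn transform by aiming mode: owner's forward, random enemy or nearest enemy.
; Enemy modes search within shoot range and rotate the shot toward the target; nothing spawns when none is found.
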(event EventBeginPlay)

(event EventTick
  (params (DeltaSeconds :type Float%20%28single-precision%29))
  (|CallParentFunction DeltaSeconds) ; This node is disabled and will not be called.\nDrag off pins to build functionality.
)

(fn Attack
  (|CallParentFunction)
  (switch Utilities|FlowControl|Switch|SwitchonE_Aiming (Variables|Default|GetAiming)
    (:NewEnumerator0
      (bind (_transform _success) (CallFunction|GetForwardTransform))
      (LocalVariables|SetLocal%20Transform _transform)
      (LocalVariables|SetLocal%20Success _success))
    (:NewEnumerator1
      (bind (_transform_2 _success_2) (CallFunction|GetRandomEnemyTransform))
      (LocalVariables|SetLocal%20Transform _transform_2)
      (LocalVariables|SetLocal%20Success _success_2))
    (:NewEnumerator2
      (bind (_transform_3 _success_3) (CallFunction|GetNearestEnemyTransform))
      (LocalVariables|SetLocal%20Transform _transform_3)
      (LocalVariables|SetLocal%20Success _success_3)))
  (if (LocalVariables|GetLocal%20Success)
    (Game|SpawnActorfromClass (Variables|Weapon|GetBullet%20Class) (LocalVariables|GetLocal%20Transform) "Undefined" 0 (Variables|Default|GetPierce) self 0)))

(fn GetForwardTransform
  (return (Transformation|GetActorTransform (Components|GetOwner)) true))

(fn GetRandomEnemyTransform
  (bind _returnvalue (Components|GetOwner))
  (bind _shoot_range (Variables|Weapon|GetShoot%20Range))
  (bind (_out_enemy _success) (CallFunction|GetRandomEnemy _shoot_range))
  (bind _returnvalue_2 (Transformation|GetActorLocation _returnvalue))
  (LocalVariables|SetLocal%20Target%20Enemy _out_enemy)
  (if _success
    (return (Math|Transform|MakeTransform _returnvalue_2 (Math|Rotator|FindLookatRotation _returnvalue_2 (Transformation|GetActorLocation (LocalVariables|GetLocal%20Target%20Enemy)))) true)
    (else
      (return "" false))))

(fn GetNearestEnemyTransform
  (bind _returnvalue (Components|GetOwner))
  (bind _returnvalue_2 (Components|GetOwner))
  (bind _shoot_range (Variables|Weapon|GetShoot%20Range))
  (bind _returnvalue_3 (Transformation|GetActorLocation _returnvalue))
  (bind _returnvalue_4 (Transformation|GetActorLocation _returnvalue_2))
  (bind (_out_enemy _success) (CallFunction|GetNearestEnemy _returnvalue_4 _shoot_range))
  (LocalVariables|SetLocal%20Target%20Enemy _out_enemy)
  (if _success
    (return (Math|Transform|MakeTransform _returnvalue_3 (Math|Rotator|FindLookatRotation _returnvalue_3 (Transformation|GetActorLocation (LocalVariables|GetLocal%20Target%20Enemy)))) true)
    (else
      (return "" false))))