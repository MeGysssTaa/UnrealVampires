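; BPC_Weapon_Harp is the weapon component for the harp in the night part of the game.
; It overrides Attack to run the parent logic and then fire through AttackShoot.
; When the shot succeeds, it plays the harp attack sound at the owner's location and returns the result.
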(event EventBeginPlay
  (|CallParentFunction) ; This node is disabled and will not be called.\nDrag off pins to build functionality.
)

(event EventTick
  (params (DeltaSeconds :type Float%20%28single-precision%29))
  (|CallParentFunction DeltaSeconds) ; This node is disabled and will not be called.\nDrag off pins to build functionality.
)

(fn Attack
  (|CallParentFunction)
  (bind _success (CallFunction|AttackShoot))
  (if _success
    (Audio|PlaySoundatLocation "/Game/Night/Weapons/Harp/S_Weapon_Harp_Attack_Cue.S_Weapon_Harp_Attack_Cue" (Transformation|GetActorLocation (Components|GetOwner)) "0, 0, 0" 1.0 1.0 0.0 0 0 0 0))
  (return _success))