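; BP_PickableCoin is a spinning gold pickup that adds its value to the saved gold, saves and destroys itself when BP_Hero touches its capsule.
; While the hero is inside MagnetArea, Tick launches the coin as a Character toward the player, pulling harder at closer range and carrying momentum from its current velocity.
; The construction script scales the capsule with GoldValue, so richer coins appear larger.
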(event OnComponentBeginOverlap(MagnetArea)
  (params (OverlappedComponent :type Primitive%20Component%20Object%20Reference) (OtherActor :type Actor%20Object%20Reference) (OtherComp :type Primitive%20Component%20Object%20Reference) (OtherBodyIndex :type Integer) (bFromSweep :type Boolean) (SweepResult :type Hit%20Result%20Structure%20%28by%20ref%29))
  (Utilities|Casting|CastToBP_Hero OtherActor)
  (Variables|Default|SetIs%20Magneting true))

(event OnComponentEndOverlap(MagnetArea)
  (params (OverlappedComponent :type Primitive%20Component%20Object%20Reference) (OtherActor :type Actor%20Object%20Reference) (OtherComp :type Primitive%20Component%20Object%20Reference) (OtherBodyIndex :type Integer))
  (Utilities|Casting|CastToBP_Hero OtherActor)
  (Variables|Default|SetIs%20Magneting false))

(event OnComponentBeginOverlap(CapsuleComponent)
  (params (OverlappedComponent :type Primitive%20Component%20Object%20Reference) (OtherActor :type Actor%20Object%20Reference) (OtherComp :type Primitive%20Component%20Object%20Reference) (OtherBodyIndex :type Integer) (bFromSweep :type Boolean) (SweepResult :type Hit%20Result%20Structure%20%28by%20ref%29))
  (bind _my_game_instance (Variables|Default|GetMy%20Game%20Instance))
  (bind _my_save (Variables|/Game/City/GI_Undeads.GI_Undeads_C|GetMy%20Save _my_game_instance))
  (Utilities|Casting|CastToBP_Hero OtherActor)
  (Variables|/Game/City/BP_Save.BP_Save_C|SetGold _my_save (+ (Variables|/Game/City/BP_Save.BP_Save_C|GetGold _my_save) (Variables|Default|GetGold%20Value)))
  (Default|SaveGame (Variables|Default|GetMy%20Game%20Instance))
  (Actor|DestroyActor))

(event EventBeginPlay
  (bind _asgi_undeads (Utilities|Casting|CastToGI_Undeads (Game|GetGameInstance)))
  (Variables|Default|SetMy%20Game%20Instance _asgi_undeads))

(event EventTick
  (params (DeltaSeconds :type Float%20%28single-precision%29))
  (Utilities|FlowControl|Sequence
    (:then_0
      (if (Variables|Default|GetIs%20Magneting)
        (CallFunction|UpdateMagnetism)))
    (:then_1
      (CallFunction|UpdateSpinningAnimation))))

(fn ConstructionScript
  (Transformation|SetRelativeScale3D (Variables|Collision|GetCapsuleComponent) (Math|Conversions|ToVector(Float) (+ (Variables|Default|GetBase%20Scale) (* (Math|Conversions|ToFloat(Integer) (Variables|Default|GetGold%20Value)) (Variables|Default|GetGold%20Value%20Size%20Scale))))))

(fn UpdateSpinningAnimation
  (Class|Actor|AddActorWorldRotation (Math|Rotator|MakeRotator 0.0 0.0 (* (Utilities|Time|GetWorldDeltaSeconds) (Variables|Default|GetSpinning%20Animation%20Speed)))))

(fn UpdateMagnetism
  (LocalVariables|SetDist%20Vec (- (Transformation|GetActorLocation (Game|GetPlayerCharacter 0)) (Transformation|GetActorLocation)))
  (Character|LaunchCharacter (+ (* (Transformation|GetVelocity) (Variables|Default|GetMagnet%20Momentum)) (* (Math|Vector|Normalize (LocalVariables|GetDist%20Vec)) (Variables|Default|GetMagnet%20Strength) (Utilities|Time|GetWorldDeltaSeconds) (- 1.0 (/ (Math|Vector|VectorLength (LocalVariables|GetDist%20Vec)) (Components|Sphere|GetScaledSphereRadius (Variables|Default|GetMagnet%20Area)))))) true true))