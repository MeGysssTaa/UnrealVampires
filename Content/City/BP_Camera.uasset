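; BP_Camera is a player-controlled camera that pans through the City part of the game.
; On BeginPlay it casts its controller to a PlayerController and registers the IMC_City Enhanced Input mapping context.
; While IA_MoveCamera triggers, it moves the actor along its local X and Y axes by the input scaled by MoveCamSpeed, without sweep or delta-time scaling.
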(event Input|EnhancedActionEvents|EnhancedInputActionIA_MoveCamera
  (params (ActionValue :type Vector%202D%20Structure) (ElapsedSeconds :type Float%20%28double-precision%29) (TriggeredSeconds :type Float%20%28double-precision%29) (InputAction :type Input%20Action%20Object%20Reference :default "/Game/City/Input/Actions/IA_MoveCamera.IA_MoveCamera"))
  (:Triggered
    (Transformation|AddActorLocalOffset (Math|Vector|MakeVector (* (.x ActionValue) (Variables|Default|GetMoveCamSpeed)) 0.0 0.0) false false)
    (Transformation|AddActorLocalOffset (Math|Vector|MakeVector 0.0 (* (.y ActionValue) (Variables|Default|GetMoveCamSpeed)) 0.0) false false)))

(event EventBeginPlay
  (bind _asplayer_controller (Utilities|Casting|CastToPlayerController (Pawn|GetController)))
  (Utilities|IsValid (PlayerController|LocalPlayerSubsystems|GetEnhancedInputLocalPlayerSubsystem _asplayer_controller)
    (:Is%20Valid
      (Input|AddMappingContext (PlayerController|LocalPlayerSubsystems|GetEnhancedInputLocalPlayerSubsystem _asplayer_controller) "/Game/City/Input/IMC_City.IMC_City" 0 "(bIgnoreAllPressedKeysUntilRelease=True,bForceImmediately=False)"))))

(fn ConstructionScript)