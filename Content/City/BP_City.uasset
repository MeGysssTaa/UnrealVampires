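; BP_City sets up the city on BeginPlay by showing the UI_City widget and restoring the player's saved buildings.
; It reads the building list from the GI_Undeads save and looks up each tag in DT_Buildings for the class to spawn.
; Each building spawns at the BP_Cell whose actor tag matches its saved "X_Y" coordinates, and that cell stores it as MyBld.
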(event EventBeginPlay
  (bind _returnvalue (UserInterface|CreateWidget "/Game/City/UI_City.UI_City_C"))
  (UserInterface|Viewport|AddtoViewport _returnvalue 0)
  (bind _asgi_undeads (Utilities|Casting|CastToGI_Undeads (Game|GetGameInstance)))
  (bind _output_get (Variables|Default|SetMy%20Game%20Instance _asgi_undeads))
  (for _array_element (Variables|/Game/City/BP_Save.BP_Save_C|GetBuildings (Variables|/Game/City/GI_Undeads.GI_Undeads_C|GetMy%20Save _output_get))
    (bind _returnvalue_2 (Utilities|GetDataTableRow "/Game/City/DT_Buildings.DT_Buildings" (Utilities|String|StringToName (.Tag (Utilities|Struct|BreakSK_Game_Building _array_element))))
      (:then
        (bind _outactors (Actor|GetAllActorsOfClasswithTag "/Game/City/BP_Cell.BP_Cell_C" (Utilities|String|StringToName (Utilities|String|Append (Utilities|String|ToString(Integer) (.X (Utilities|Struct|BreakSK_Game_Building _array_element))) "_" (Utilities|String|ToString(Integer) (.Y (Utilities|Struct|BreakSK_Game_Building _array_element)))))))
        (bind _returnvalue_3 (Game|SpawnActorfromClass (.Class (Utilities|Struct|BreakSK_Building _returnvalue_2)) (Transformation|GetActorTransform (Utilities|Array|Get(acopy) _outactors)) "Undefined" 0 0))
        (Variables|/Game/City/BP_Cell.BP_Cell_C|SetMy%20Bld (Utilities|Array|Get(acopy) _outactors) _returnvalue_3)))))

(event Collision|EventActorBeginOverlap
  (params (OtherActor :type Actor%20Object%20Reference)))

(event EventTick
  (params (DeltaSeconds :type Float%20%28single-precision%29)))

(fn ConstructionScript)