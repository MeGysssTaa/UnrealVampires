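; BP_Cell is a city grid cell that places the selected card's building when clicked.
; On BeginPlay it caches the GI_Undeads game instance and tags itself with its "X:Y" coordinates so saved buildings can be restored to it.
; A click on an empty cell spawns the BldPrms class at the cell's transform, appends a level-one building record to the save, and saves the game.
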(event OnClicked(Cube)
  (params (TouchedComponent :type Primitive%20Component%20Object%20Reference) (ButtonPressed :type Key%20Structure))
  (bind _bld_prms (Variables|Default|GetBld%20Prms))
  (bind (_tag _icon _class) (Utilities|Struct|BreakSK_Building _bld_prms))
  ;[0.4573 0.7705 1] Place the selected card's building in this cell on click
  (Utilities|IsValid (Variables|Default|GetMy%20Bld)
    (:Is%20Not%20Valid
      (bind _returnvalue (Game|SpawnActorfromClass _class (Transformation|GetActorTransform) "Undefined" 0 0))
      (Variables|Default|SetMy%20Bld _returnvalue)
      (Utilities|Array|Add (Variables|/Game/City/BP_Save.BP_Save_C|GetBuildings (Variables|/Game/City/GI_Undeads.GI_Undeads_C|GetMy%20Save (Variables|Default|GetMy%20Game%20Instance))) (Utilities|Struct|MakeSK_Game_Building _tag 1 (Variables|Default|GetX) (Variables|Default|GetY)))
      (Default|SaveGame (Variables|Default|GetMy%20Game%20Instance)))))

(event EventBeginPlay
  ;[1 0.8287 0.2811] Enable restoring this cell's state/building from save file
  (Utilities|FlowControl|Sequence
    (:then_0
      (bind _asgi_undeads (Utilities|Casting|CastToGI_Undeads (Game|GetGameInstance)))
      (Variables|Default|SetMy%20Game%20Instance _asgi_undeads))
    (:then_1
      (Utilities|Array|Add (Variables|Actor|GetTags) (Utilities|String|StringToName (Utilities|String|Append (Utilities|String|ToString(Integer) (Variables|Default|GetX)) ":" (Utilities|String|ToString(Integer) (Variables|Default|GetY))))))))

(fn ConstructionScript)